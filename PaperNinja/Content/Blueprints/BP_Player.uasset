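; Player character Blueprint that handles Enhanced Input movement, yaw-only look, sprint and a simple one-hit death.
; Movement follows the camera's forward and right vectors, sprint switches max walk speed, and jumping from near standstill is delayed as a wind-up.
; Any damage, including self-damage from the force-kill input, disables movement once via DoOnce and prints a death message.
; Tick draws a debug arrow of the current velocity.
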(event `self.ReceiveTick`
  (params (DeltaSeconds :type "Float (single-precision)"))
  (bind _returnvalue (`self.K2_GetActorLocation`))
  (`KismetSystemLibrary.DrawDebugArrow` _returnvalue (+ _returnvalue (`self.GetVelocity`)) 2.0 (struct :`R` 0.229042 :`G` 1.0 :`B` 0.986736 :`A` 1.0) 0.0 2.0))

(event `self.ReceiveAnyDamage`
  (params (Damage :type "Float (single-precision)") (DamageType :type "DamageType Object Reference") (InstigatedBy :type "Controller Object Reference") (DamageCauser :type "Actor Object Reference"))
  (`/Engine/EditorBlueprintResources/StandardMacros.DoOnce` false ; 死亡処理は一度だけ実行する
    (:`Completed`
      (`KismetSystemLibrary.PrintString` "Died！")
      (`CharacterMovementComponent.DisableMovement` (`self.CharacterMovement`)))))

(event `EnhancedInput|/Game/Inputs/IA_Jump`
  (params (ActionValue :type Boolean) (ElapsedSeconds :type "Float (double-precision)") (TriggeredSeconds :type "Float (double-precision)") (InputAction :type "InputAction Object Reference" :default "/Game/Inputs/IA_Jump.IA_Jump"))
  ;[1 1 1] ジャンプ操作の制御。静止時はタメジャンプする
  (:`Triggered`
    (if (`self.CanJump`)
      (if (not (>= (`KismetMathLibrary.VSizeXY` (`self.GetVelocity`)) 10.0))
        (`KismetSystemLibrary.Delay` 0.3))
      (`self.Jump`))))

(event `EnhancedInput|/Game/Inputs/IA_Look`
  (params (ActionValue :type "Vector2D Structure") (ElapsedSeconds :type "Float (double-precision)") (TriggeredSeconds :type "Float (double-precision)") (InputAction :type "InputAction Object Reference" :default "/Game/Inputs/IA_Look.IA_Look"))
  (:`Triggered`
    (`self.AddControllerYawInput` (`KismetMathLibrary.BreakVector2D` ActionValue))))

(event `EnhancedInput|/Game/Inputs/IA_Sprint`
  (params (ActionValue :type Boolean) (ElapsedSeconds :type "Float (double-precision)") (TriggeredSeconds :type "Float (double-precision)") (InputAction :type "InputAction Object Reference" :default "/Game/Inputs/IA_Sprint.IA_Sprint"))
  (bind _charactermovement (`self.CharacterMovement`))
  (:`Triggered`
    (set `CharacterMovementComponent.MaxWalkSpeed` 200.0 _charactermovement) ; スプリント時のスピード
  )
  (:`Completed`
    (set `CharacterMovementComponent.MaxWalkSpeed` 75.0 _charactermovement) ; 通常歩行時のスピード
  ))

(event `EnhancedInput|/Game/Inputs/IA_Move`
  (params (ActionValue :type "Vector2D Structure") (ElapsedSeconds :type "Float (double-precision)") (TriggeredSeconds :type "Float (double-precision)") (InputAction :type "InputAction Object Reference" :default "/Game/Inputs/IA_Move.IA_Move"))
  (bind (_x _y) (`KismetMathLibrary.BreakVector2D` ActionValue))
  (:`Triggered`
    (`self.AddMovementInput` (`SceneComponent.GetForwardVector` (`self.Camera`)) _y) ; 前後移動
    (`self.AddMovementInput` (`SceneComponent.GetRightVector` (`self.Camera`)) _x) ; 左右移動
  ))

(event `EnhancedInput|/Game/Inputs/IA_Forcekill`
  (params (ActionValue :type Boolean) (ElapsedSeconds :type "Float (double-precision)") (TriggeredSeconds :type "Float (double-precision)") (InputAction :type "InputAction Object Reference" :default "/Game/Inputs/IA_Forcekill.IA_Forcekill"))
  (:`Triggered`
    (`GameplayStatics.ApplyDamage` self 1.0 null self) ; 自分自身にダメージを適用
  ))

(fn `UserConstructionScript`)